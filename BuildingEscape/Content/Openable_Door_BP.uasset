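; Openable door actor that swings open and shut when its OpenDoor component requests it.
; On BeginPlay it stores the starting rotation, then a timeline drives a yaw offset combined with that rotation to turn the whole actor.
; A timeline event track plays the door lock sound at the actor's location, and close requests play the same timeline in reverse.
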(event OnOpenRequest(OpenDoor)
  (bind _dooryaw (Timeline|Timeline_0 Play)
    (:Update
      (Transformation|SetActorRotation (Math|Rotator|CombineRotators (Variables|Default|GetStartRotation) (Math|Rotator|MakeRotator 0.0 0.0 _dooryaw))))
    (:Sound%20Timing
      (Audio|PlaySoundatLocation "/Game/Audio/door-lock.door-lock" (Transformation|GetActorLocation)))))

(event OnCloseRequest(OpenDoor)
  (bind _dooryaw (Timeline|Timeline_0 Reverse)
    (:Update
      (Transformation|SetActorRotation (Math|Rotator|CombineRotators (Variables|Default|GetStartRotation) (Math|Rotator|MakeRotator 0.0 0.0 _dooryaw))))
    (:Sound%20Timing
      (Audio|PlaySoundatLocation "/Game/Audio/door-lock.door-lock" (Transformation|GetActorLocation)))))

(event EventBeginPlay
  (Variables|Default|SetStartRotation (Transformation|GetActorRotation)))

(event Collision|EventActorBeginOverlap
  (params (OtherActor :type Actor%20Object%20Reference)))

(event EventTick
  (params (DeltaSeconds :type Float%20%28single-precision%29)))

(fn ConstructionScript)